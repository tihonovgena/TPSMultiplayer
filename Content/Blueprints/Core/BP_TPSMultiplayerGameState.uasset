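; Game State Blueprint for a multiplayer third-person shooter that tracks match state and remaining match time.
; On BeginPlay, only the authority starts the match, recording the server world time and setting the match state enum.
; Time left is derived on demand from server world time and clamped between zero and the match length, so no ticking countdown is needed.
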(event `self.ReceiveBeginPlay`
  (`/Engine/EditorBlueprintResources/ActorMacros.Switch Has Authority`
    (:`Authority`
      (`self.StartMatch`))))

(fn `GetGameTimeLeft`
  (returns (Time :type "Float (double-precision)"))
  (return (`self.GetMatchLeftTime`)))

(fn `GetMatchLeftTime`
  (returns (ReturnValue :type "Float (double-precision)"))
  (return (`KismetMathLibrary.FClamp` (- (`self.MatchTime`) (- (`self.GetServerWorldTimeSeconds`) (`self.StartMatchTime`))) 0.0 (`self.MatchTime`))))

(fn `GetMatchState`
  (returns (State :type "/Game/Blueprints/Core/Misc/EMatchState Enum"))
  (return (`self.MatchStarted`)))

(fn `StartMatch`
  (set `self.StartMatchTime` (`self.GetServerWorldTimeSeconds`))
  (set `self.MatchStarted` "NewEnumerator1"))

(fn `UserConstructionScript`)