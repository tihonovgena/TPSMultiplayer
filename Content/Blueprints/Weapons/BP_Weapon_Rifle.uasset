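; Rifle weapon Blueprint that extends a parent weapon with automatic hitscan fire.
; DoShoot fires immediately, then repeats Shoot on a looping timer until StopShoot clears it.
; Each shot runs parent logic, then traces from the muzzle toward a point along the owning character's controller view, damaging the hit actor and drawing debug lines.
; Without ammo, Shoot stops firing and signals for a reload, which defers to the parent.
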(event `DoShoot_1`
  ;[1 1 1] Shooting
)

(event `StopShoot_1`
  ;[1 1 1] Shooting
)

(fn `DoShoot`
  (`self.Shoot`)
  (bind _returnvalue (`KismetSystemLibrary.K2_SetTimer` null "Shoot" (`self.ShotFrequency`) true))
  (set `self.ShootTimerHandle` _returnvalue))

(fn `GetOwnerController`
  (returns (ReturnValue :type "Controller Object Reference"))
  (bind _aspawn (cast `Pawn` (`self.GetOwner`)))
  (return (`Pawn.GetController` _aspawn)))

(fn `Reload`
  (returns (ReturnValue :type Boolean))
  (bind _returnvalue (`parent.Reload`))
  (return _returnvalue))

(fn `Shoot`
  (if (`self.HasAmmo`)
    (`parent.Shoot`)
    (`self.TraceShot`)
    (else
      (`self.StopShoot`)
      (`self.OnRequireReload`))))

(fn `StopShoot`
  (`KismetSystemLibrary.K2_ClearAndInvalidateTimerHandle` (`self.ShootTimerHandle`)))

(fn `TraceShot`
  (bind _asbpi_third_person_character (cast `/Game/Blueprints/Interfaces/BPI_ThirdPersonCharacter` (`self.GetOwner`)))
  (bind (_location _rotation) (`/Game/Blueprints/Interfaces/BPI_ThirdPersonCharacter.GetControllerViewPoint` _asbpi_third_person_character))
  (bind (_outhit _returnvalue) (`KismetSystemLibrary.LineTraceSingle` (`self.GetMuzzleSocketLocation`) (+ _location (* (`KismetMathLibrary.GetForwardVector` _rotation) (`self.ShotDistance`))) "TraceTypeQuery3" false (`|MakeArray` (`self.GetOwner`)) "ForDuration"))
  (if _returnvalue
    (`GameplayStatics.ApplyDamage` (`.HitActor` (`GameplayStatics.BreakHitResult` _outhit)) (`self.GetDamage`) (`self.GetOwnerController`))))

(fn `UserConstructionScript`)