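; BP_Projectile is a replicated weapon projectile that flies along a set Direction and deals radial damage on impact.
; The server sets velocity from Direction and initial speed on BeginPlay, while OnRep_Direction applies the same velocity on clients.
; On a server-side hit against anything but its owner, it applies full radial damage credited to the owning pawn's controller, draws a debug sphere and destroys itself.
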(event `self.ReceiveBeginPlay`
  (`self.SetLifeSpan` 10.0)
  (`/Engine/EditorBlueprintResources/ActorMacros.Switch Has Authority`
    (:`Authority`
      (`self.SetupVelocity`))))

(event `self.ReceiveHit`
  (params (MyComp :type "PrimitiveComponent Object Reference") (Other :type "Actor Object Reference") (OtherComp :type "PrimitiveComponent Object Reference") (bSelfMoved :type Boolean) (HitLocation :type "Vector Structure") (HitNormal :type "Vector Structure") (NormalImpulse :type "Vector Structure") (Hit :type "HitResult Structure (by ref)"))
  (bind _damageradius (`self.DamageRadius`))
  (`/Engine/EditorBlueprintResources/ActorMacros.Switch Has Authority`
    (:`Authority`
      (if (!= Other (`self.GetOwner`))
        (`GameplayStatics.ApplyRadialDamage` :`BaseDamage` (`self.Damage`) :`Origin` HitLocation :`DamageRadius` _damageradius :`DamageCauser` null :`InstigatedByController` (`self.GetOwnerController`) :`bDoFullDamage` true)
        (`KismetSystemLibrary.DrawDebugSphere` (`.Location` (`GameplayStatics.BreakHitResult` Hit)) _damageradius 12 (struct :`R` 1.0 :`G` 1.0 :`B` 1.0 :`A` 1.0) 10.0 2.0)
        (`self.K2_DestroyActor`)))))

(fn `GetOwnerController`
  (returns (ReturnValue :type "Controller Object Reference"))
  (bind _aspawn (cast `Pawn` (`self.GetOwner`)))
  (return (`Pawn.GetController` _aspawn)))

(fn `OnRep_Direction`
  (`self.SetupVelocity`))

(fn `SetDirection`
  (params (Direction :type "Vector Structure"))
  (set `self.Direction` Direction))

(fn `SetupVelocity`
  (bind _projectilemovement (`self.ProjectileMovement`))
  (set `MovementComponent.Velocity` (* (`self.Direction`) (`ProjectileMovementComponent.InitialSpeed` _projectilemovement)) _projectilemovement))

(fn `UserConstructionScript`)