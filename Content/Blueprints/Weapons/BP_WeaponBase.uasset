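; Base weapon Blueprint that exposes muzzle position, damage and ammunition data through getter functions.
; The muzzle location comes from a named socket on the weapon mesh, and damage is read directly from a variable.
; Current ammo, clip and default ammo getters forward to functions defined outside these graphs.
; The event graph and construction script hold no logic.
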(fn `GetAmmoAmount`
  (returns (Ammo :type Integer))
  (return (`self.GetAmmo`)))

(fn `GetClipsAmount`
  (returns (Clips :type Integer))
  (return (`self.GetClips`)))

(fn `GetDamage`
  (returns (Damage :type "Float (double-precision)"))
  (return (`self.Damage`)))

(fn `GetDefaultAmmoAmount`
  (returns (Default :type Integer))
  (return (`self.GetDefaultAmmo`)))

(fn `GetMuzzleSocketLocation`
  (returns (Location :type "Vector Structure"))
  (return (`SceneComponent.GetSocketLocation` (`self.WeaponMesh`) (`self.MuzzleSocketName`))))

(fn `UserConstructionScript`)