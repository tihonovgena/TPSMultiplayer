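; BP_Weapon_Launcher is a projectile launcher weapon that fires explosive-style shots with area damage.
; DoShoot overrides the parent weapon's firing: with ammo it runs the parent logic and then Shoot, otherwise it signals that a reload is required.
; Shoot spawns a BP_Projectile at the muzzle socket, passing the aim direction, weapon damage, damage radius and the weapon's owner.
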(fn `DoShoot`
  (if (`self.HasAmmo`)
    (`parent.DoShoot`)
    (`self.Shoot`)
    (else
      (`self.OnRequireReload`))))

(fn `Shoot`
  (bind _returnvalue (`self.GetMuzzleSocketRotation`))
  (`|SpawnActorFromClass` "/Game/Blueprints/Weapons/Ammo/BP_Projectile.BP_Projectile_C" (`KismetMathLibrary.MakeTransform` (`self.GetMuzzleSocketLocation`) _returnvalue) "AlwaysSpawn" "MultiplyWithRoot" (`self.GetOwner`) (`KismetMathLibrary.GetForwardVector` _returnvalue) (`self.GetDamage`) (`self.DamageRadius`) null))

(fn `UserConstructionScript`)